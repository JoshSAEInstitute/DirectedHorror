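; BP_Immobile is a character that chases the player while unseen and freezes while being rendered, in the style of a Weeping Angel.
; Every tick, it checks whether its mesh was recently rendered.
; If not, it uses SimpleMoveToLocation toward the player and plays animation at normal rate.
; Once rendered, an IsMoving flag triggers a single stop that halts the controller, zeroes velocity and pauses animation through the mesh's global rate scale.
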(event `self.ReceiveTick`
  (params (DeltaSeconds :type "Float (single-precision)"))
  (if (`PrimitiveComponent.WasRecentlyRendered` (`self.Mesh`) 0.05)
    (if (`self.isMoving?`)
      ;[1 1 1] Stops Movement and Animation
      (`Controller.StopMovement` (`self.GetController`))
      (set `self.isMoving?` false)
      (set `SkeletalMeshComponent.GlobalAnimRateScale` 0.0 (`self.Mesh`))
      (set `MovementComponent.Velocity` (0.0 0.0 0.0) (`self.CharacterMovement`)))
    (else
      (`AIBlueprintHelperLibrary.SimpleMoveToLocation` (`self.GetController`) (`self.K2_GetActorLocation` (`GameplayStatics.GetPlayerCharacter` 0)))
      (set `self.isMoving?` true)
      (set `SkeletalMeshComponent.GlobalAnimRateScale` 1.0 (`self.Mesh`)))))

(fn `UserConstructionScript`)