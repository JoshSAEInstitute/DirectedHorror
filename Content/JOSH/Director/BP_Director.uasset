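; BP_Director is a horror game director that paces scares through a tension meter and spawns keys for exit gates at BeginPlay.
; Tick raises tension while a few Immobiles are in view, otherwise decays it and checks thresholds.
; Low tension spawns Immobiles at random reachable points and adds tension, while high tension randomly destroys one.
; A jumpscare event flashes a widget with sound and boosts tension; the EventRecentlyTriggered cooldown setter is unconnected.
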(event `Spawn Immobile`
  ;[0 0.9216 1] Immobile Spawner
  (`|SpawnActorFromClass` "/Game/JOSH/Immobile/BP_Immobile/BP_Immobile.BP_Immobile_C" (`KismetMathLibrary.MakeTransform` (`NavigationSystemV1.K2_GetRandomReachablePointInRadius` (`SceneComponent.K2_GetComponentLocation` (`self.DefaultSceneRoot`)) 5000.0 null null) (`KismetMathLibrary.MakeRotator` 0.0 0.0 (`KismetMathLibrary.RandomFloatInRange` 0.0 360.0))) "Undefined" "MultiplyWithRoot" null null))

(event `Destroy Random Immobile`
  ;[1 1 1] Testing Purposes
  (bind _outactors (`GameplayStatics.GetAllActorsOfClass` "/Game/JOSH/Immobile/BP_Immobile/BP_Immobile.BP_Immobile_C" :!label _label))
  (bind _output_get (set `self.ImmobileRef` _outactors))
  (for (_ _array_index) _output_get
    _)
  (`self.K2_DestroyActor` (`|GetArrayItem` (`self.ImmobileRef`) (`KismetMathLibrary.RandomIntegerInRange` 0 _array_index)))
  (`KismetArrayLibrary.Array_Clear` (`self.ImmobileRef`)))

(event `High Tension Event`
  (`|MultiGate` true true
    (:`Out 0`
      (goto _label))))

(event `JumpScareImmobile`
  ;[0 0.9216 1] Immobile JumpScare
  (bind _returnvalue (`|CreateWidget` "/Game/JOSH/Immobile/WBP_JumpscareImmobile.WBP_JumpscareImmobile_C"))
  (`UserWidget.AddToViewport` _returnvalue 0)
  (`GameplayStatics.PlaySound2D` "/Game/JOSH/Immobile/Sound_Immobile_1.Sound_Immobile_1" 1.0 1.0 0.0 null null)
  (`KismetSystemLibrary.Delay` 0.2)
  (`WidgetLayoutLibrary.RemoveAllWidgets`)
  (set `self.TensionBarMetre` (+ (`self.TensionBarMetre`) 20.0)))

(event `Immobile Amount`
  ;[0 0.9216 1] Immobile Amount
  (`KismetSystemLibrary.PrintString` (`KismetStringLibrary.Concat_StrStr` "Immobile amount: " (`KismetStringLibrary.Conv_IntToString` (`self.ImmobileAmount`))) true true (struct :`R` 0.016101 :`G` 1.0 :`A` 1.0) 0.01)
  (if (< (`self.ImmobileAmount`) 0)
    (set `self.ImmobileAmount` 0)))

(event `Low Tension Event`
  (`|MultiGate` true true
    (:`Out 0`
      _)
    (:`Out 1`
      _)
    (:`Out 2`
      _))
  (`self.Spawn Immobile`)
  (set `self.TensionBarMetre` (+ (`self.TensionBarMetre`) 15.0)))

(event `LightTensionIncrease`
  ;[1 0.4275 0] Light Tension Increase
  (set `self.TensionBarMetre` (+ (`self.TensionBarMetre`) 0.01))
  (`KismetSystemLibrary.PrintString` "Light Tension" true true (struct :`R` 1.0 :`G` 0.82651 :`A` 1.0) 0.01))

(event `self.ReceiveTick`
  (params (DeltaSeconds :type "Float (single-precision)"))
  ;[1 1 1] Event Tick
  (`self.Immobile Amount`)
  (`KismetSystemLibrary.PrintString` (`KismetStringLibrary.Concat_StrStr` "Tension Bar amount: " (`KismetStringLibrary.Conv_DoubleToString` (`self.TensionBarMetre`))) true true (struct :`R` 1.0 :`B` 0.011267 :`A` 1.0) 0.01)
  ;;[1 1 1] Immobile Amount Checker
  (if (`self.ImmobileInView?`)
    (if (<= (`self.ImmobileAmount`) 2)
      (`self.LightTensionIncrease`))
    (else
      (`self.TB_FinalEvent`))))

(event `TB_FinalEvent`
  ;[1 0.4275 0] Tension Bar Check
  (set `self.TensionBarMetre` (- (`self.TensionBarMetre`) 0.005))
  (if (`self.EventRecentlyTriggered`)
    _
    (elif (<= (`self.TensionBarMetre`) 25.0)
      (`self.Low Tension Event`)
      (elif (>= (`self.TensionBarMetre`) 75.0)
        (`self.High Tension Event`)))))

(event `self.ReceiveBeginPlay`
  (bind _output (`|GetArrayItem` (`self.KeyLocations`) (`self.RandomNumber`)))
  (`|ExecutionSequence`
    (:`then_0`
      (set `self.TensionBarMetre` 25.0)
      (bind _returnvalue (`GameplayStatics.GetActorOfClass` "/Game/JOSH/Terror/BP_Terror.BP_Terror_C"))
      (set `self.Terror` _returnvalue))
    (:`then_1`
      ;[1 1 1] Exit Door
      (bind _outactors (`GameplayStatics.GetAllActorsOfClass` "/Game/JOSH/LockGateKeys/ExitGate.ExitGate_C"))
      (for _array_element _outactors
        (set `self.RandomNumber` (`KismetMathLibrary.RandomInteger` 2))
        (`KismetSystemLibrary.PrintString` (`KismetStringLibrary.Concat_StrStr` "Number picked: " (`KismetStringLibrary.Conv_IntToString` (`self.RandomNumber`)) " > Location spawned: " (`KismetStringLibrary.Conv_TransformToString` _output)) true true (struct :`G` 0.66 :`B` 1.0 :`A` 1.0) 10.0)
        (bind _returnvalue_2 (`|SpawnActorFromClass` "/Game/JOSH/LockGateKeys/KeySpawner.KeySpawner_C" _output "Undefined" "MultiplyWithRoot" null null))
        (set `/Game/JOSH/LockGateKeys/KeySpawner.ExitGateRef` _array_element _returnvalue_2)))))

(fn `UserConstructionScript`)