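; A game director Blueprint that tracks a tension meter and places key spawners for the level's exit gates.
; At start it sets the meter, then spawns a KeySpawner for each ExitGate at a randomly chosen one of the first two KeyLocations and passes it that gate.
; IncreaseTensionBar raises the meter while Tick lowers it per frame, with debug prints showing the values.
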(event `Increase Tension Bar`
  (set `self.TensionBarMetre` (+ (`self.TensionBarMetre`) 1.0))
  (`KismetSystemLibrary.PrintString` "Increased"))

(event `self.ReceiveTick`
  (params (DeltaSeconds :type "Float (single-precision)"))
  (`KismetSystemLibrary.PrintString` (`KismetStringLibrary.Concat_StrStr` "Tension Bar amount: " (`KismetStringLibrary.Conv_DoubleToString` (`self.TensionBarMetre`))) true true (struct :`R` 1.0 :`B` 0.011267 :`A` 1.0) 0.01)
  (set `self.TensionBarMetre` (- (`self.TensionBarMetre`) 0.005)))

(event `self.ReceiveBeginPlay`
  (bind _output (`|GetArrayItem` (`self.KeyLocations`) (`self.RandomNumber`)))
  (`|ExecutionSequence`
    (:`then_0`
      (set `self.TensionBarMetre` 25.0))
    (:`then_1`
      ;[1 1 1] Exit Door
      (bind _outactors (`GameplayStatics.GetAllActorsOfClass` "/Game/JOSH/LockGateKeys/ExitGate.ExitGate_C"))
      (for _array_element _outactors
        (set `self.RandomNumber` (`KismetMathLibrary.RandomInteger` 2))
        (`KismetSystemLibrary.PrintString` (`KismetStringLibrary.Concat_StrStr` "Number picked: " (`KismetStringLibrary.Conv_IntToString` (`self.RandomNumber`)) " > Location spawned: " (`KismetStringLibrary.Conv_TransformToString` _output)) true true (struct :`G` 0.66 :`B` 1.0 :`A` 1.0) 10.0)
        (bind _returnvalue (`|SpawnActorFromClass` "/Game/JOSH/LockGateKeys/KeySpawner.KeySpawner_C" _output "Undefined" "MultiplyWithRoot" null null))
        (set `/Game/JOSH/LockGateKeys/KeySpawner.ExitGateRef` _array_element _returnvalue)))))

(fn `UserConstructionScript`)