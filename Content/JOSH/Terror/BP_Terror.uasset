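; BP_Terror is an AI-driven monster that can be called to a noise and jumpscares the player on contact.
; When notified, it sets a called flag and the noise location as target in its AI controller's blackboard.
; It plays an attached laugh on spawn and caches BP_Director.
; Player overlap with its jumpscare collision triggers the Director's Terror jumpscare and destroys it; TensionBarIncrease is an empty stub.
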(event `I Have Been Notified`
  (bind _returnvalue (`AIBlueprintHelperLibrary.GetBlackboard` (`AIBlueprintHelperLibrary.GetAIController` self)))
  (`BlackboardComponent.SetValueAsBool` _returnvalue "hasBeenCalled?" true)
  (`BlackboardComponent.SetValueAsVector` _returnvalue "TargetLocation" (`self.NoiseLocationRef`)))

(event `self.ReceiveBeginPlay`
  (bind _mesh (`self.Mesh`))
  (bind _returnvalue (`GameplayStatics.GetActorOfClass` "/Game/JOSH/Director/BP_Director.BP_Director_C"))
  (set `self.Director` _returnvalue)
  (`GameplayStatics.SpawnSoundAttached` "/Game/JOSH/Terror/TerrorLaugh.TerrorLaugh" _mesh "None" (`SceneComponent.K2_GetComponentLocation` _mesh) (struct) "SnapToTarget" false 1.0 1.0 0.0 null null))

(event `self.CollisionJumpscare.OnComponentBeginOverlap`
  (params (OverlappedComponent :type "PrimitiveComponent Object Reference") (OtherActor :type "Actor Object Reference") (OtherComp :type "PrimitiveComponent Object Reference") (OtherBodyIndex :type Integer) (bFromSweep :type Boolean) (SweepResult :type "HitResult Structure (by ref)"))
  (cast `/Game/FirstPerson/Blueprints/BP_FirstPersonCharacter` OtherActor)
  (`KismetSystemLibrary.PrintString` "Hello" true true (struct :`R` 0.051346 :`B` 1.0 :`A` 1.0))
  (bind _asbp_director (cast `/Game/JOSH/Director/BP_Director` (`self.Director`)))
  (`/Game/JOSH/Director/BP_Director.JumpScareTerror` _asbp_director)
  (`self.K2_DestroyActor`))

(fn `TensionBarIncrease`
  (params (Increase :type "Float (double-precision)" :default 0.0))
  (return))

(fn `UserConstructionScript`)